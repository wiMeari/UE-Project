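; BP_CameraController manages a pair of player cameras separated by a fixed height difference and feeds their transforms to scene captures.
; Each tick it mirrors the player camera above or below, based on height, then passes both transforms to BP_SceneCapture and BP_PlayerSceneCapture actors.
; EventCameraSwitch moves the player camera to the other camera's position.
; LerpCamera eases toward TargetLocation with separate XY and Z speeds, but is not called here.
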(event Custom|EventCameraSwitch
  (CallFunction|SwitchCameraLocation))

(event EventBeginPlay
  (bind _returnvalue (Actor|GetActorOfClass "/Game/T/Actor/BP_SceneCapture.BP_SceneCapture_C"))
  (Variables|Default|SetPlayerSceneCaptureActor _returnvalue)
  (bind _returnvalue_2 (Actor|GetActorOfClass "/Game/T/Actor/BP_PlayerSceneCapture.BP_PlayerSceneCapture_C"))
  (Variables|Default|SetCurrentPlayerSceneCapture _returnvalue_2))

(event Collision|EventActorBeginOverlap
  (params (OtherActor :type Actor%20Object%20Reference)))

(event EventTick
  (params (DeltaSeconds :type Float%20%28single-precision%29))
  (CallFunction|UpdateAnotherCameraLocation)
  (bind _playerscenecaptureactor (Variables|Default|GetPlayerSceneCaptureActor)
    (:then
      (Variables|/Script/TeamProject.PlayerSceneCapture|SetTargetCameraTransform _playerscenecaptureactor (Transformation|GetActorTransform (Variables|Default|GetAnotherPlayerCameraActor)))
      (bind _currentplayerscenecapture (Variables|Default|GetCurrentPlayerSceneCapture)
        (:then
          (Variables|/Script/TeamProject.PlayerSceneCapture|SetTargetCameraTransform _currentplayerscenecapture (Transformation|GetActorTransform (Variables|Default|GetPlayerCameraActor))))
        (:else)))
    (:else)))

(fn ConstructionScript)

(fn LerpCamera
  (params (DeltaTime :type Float%20%28double-precision%29))
  (bind _playercameraactor (Variables|Default|GetPlayerCameraActor))
  (bind _targetlocation (Variables|Default|GetTargetLocation))
  (bind _xyinterpspeed (Variables|Default|GetXYInterpSpeed))
  (bind _returnvalue (Transformation|GetActorLocation _playercameraactor))
  (bind _returnvalue_2 (Math|Vector|MakeVector (.x _targetlocation) (.y _targetlocation) 0.0))
  (bind _returnvalue_3 (Math|Vector|MakeVector (.x _returnvalue) (.y _returnvalue) 0.0))
  (bind _returnvalue_4 (Math|Interpolation|VInterpTo _returnvalue_3 _returnvalue_2 DeltaTime _xyinterpspeed))
  (if true
    (Transformation|SetActorLocation (Variables|Default|GetPlayerCameraActor) (Math|Vector|MakeVector (.x _returnvalue_4) (.y _returnvalue_4) (Math|Interpolation|FInterpTo (.z _returnvalue) (.z _targetlocation) DeltaTime (Variables|Default|GetZInterpSpeed))) false false)))

(fn UpdateAnotherCameraLocation
  (bind _playercameraactor (Variables|Default|GetPlayerCameraActor))
  (bind _playercameraactor_2 (Variables|Default|GetPlayerCameraActor))
  (bind _returnvalue (Transformation|GetActorTransform _playercameraactor_2))
  (bind _returnvalue_2 (Transformation|GetActorTransform _playercameraactor))
  (Variables|Default|GetAnotherPlayerCameraActor
    (:then
      (bind _playercameraactor_3 (Variables|Default|GetPlayerCameraActor)
        (:then
          (if (>= (.z (Transformation|GetActorLocation _playercameraactor_3)) (Variables|地图参数|GetCameraHeightDifference))
            (Transformation|SetActorTransform (Variables|Default|GetAnotherPlayerCameraActor) (Math|Transform|MakeTransform (Math|Vector|MakeVector (.x (.location _returnvalue_2)) (.y (.location _returnvalue_2)) (- (.z (.location _returnvalue_2)) (Variables|地图参数|GetCameraHeightDifference))) (.rotation _returnvalue_2) (.scale _returnvalue_2)))
            (else
              (Transformation|SetActorTransform (Variables|Default|GetAnotherPlayerCameraActor) (Math|Transform|MakeTransform (Math|Vector|MakeVector (.x (.location _returnvalue)) (.y (.location _returnvalue)) (+ (.z (.location _returnvalue)) (Variables|地图参数|GetCameraHeightDifference))) (.rotation _returnvalue) (.scale _returnvalue)))))
          (return))
        (:else)))
    (:else)))

(fn SwitchCameraLocation
  (bind _anotherplayercameraactor (Variables|Default|GetAnotherPlayerCameraActor)
    (:then
      (bind _playercameraactor (Variables|Default|GetPlayerCameraActor)
        (:then
          (bind _output_get (LocalVariables|SetPlayerCameraLocation (Transformation|GetActorLocation _playercameraactor)))
          (bind _output_get_2 (LocalVariables|SetAnotherCameraLocation (Transformation|GetActorLocation _anotherplayercameraactor)))
          (bind (_outfirstvector _outsecondvector) (Class|TPFunctionLibrary|SwapPlaces _output_get _output_get_2))
          (Transformation|SetActorLocation (Variables|Default|GetPlayerCameraActor) _outfirstvector false false)
          (LocalVariables|SetPlayerCameraLocation _outfirstvector)
          (LocalVariables|SetAnotherCameraLocation _outsecondvector)
          (return))
        (:else)))
    (:else)))