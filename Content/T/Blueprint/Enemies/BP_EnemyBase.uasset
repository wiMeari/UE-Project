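; Base enemy Blueprint handling chase speed, melee attacks, hit reactions and death, with combat facing and knockback constrained to the world Y axis.
; Tick switches walk speed on IsChase, while Attack snaps yaw along Y, halts movement, waits a random interval, then plays a montage whose end restores attacking and movement.
; GetHit plays a sound and launches the enemy away from the hitter.
; Death stops the weapon's BoxTrace timer and destroys the actor after a delay.
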(event EventBeginPlay)

(event Collision|EventActorBeginOverlap
  (params (OtherActor :type Actor%20Object%20Reference)))

(event EventTick
  (params (DeltaSeconds :type Float%20%28single-precision%29))
  (bind _charactermovement (Variables|Character|GetCharacterMovement))
  (|CallParentFunction DeltaSeconds)
  (if (Variables|Default|GetIsChase)
    (Variables|/Script/Engine.CharacterMovementComponent|SetMaxWalkSpeed _charactermovement (Variables|Default|Get最大行走速度))
    (else
      (Variables|/Script/Engine.CharacterMovementComponent|SetMaxWalkSpeed _charactermovement (Variables|Default|Get最小行走速度)))))

(event EventGetHit
  (params (Damage :type Float%20%28single-precision%29) (HitDirection :type Vector%20%28by%20ref%29 :default "0, 0, 0") (Hitter :type Actor%20Object%20Reference))
  (|CallParentFunction Damage HitDirection Hitter)
  (Audio|PlaySoundatLocation "/Game/T/Audio/GetHit/MS_EnemyGetHit.MS_EnemyGetHit" (Transformation|GetActorLocation) "0, 0, 0" 1.0 1.0 0.0 0 0 0 0)
  (bind _launchvelocity (CallFunction|CalcLaunchVelocity Hitter))
  (Character|LaunchCharacter _launchvelocity false false))

(event EventDeath
  (|CallParentFunction)
  (Variables|Default|SetIsDeath true)
  (bind _asbp_base_weapon (Utilities|Casting|CastToBP_BaseWeapon (Variables|/Script/Engine.ChildActorComponent|GetChildActor (Variables|Default|GetWeaponComponent))))
  (Utilities|Time|ClearTimerbyFunctionName _asbp_base_weapon "BoxTrace")
  (Utilities|FlowControl|Delay 3.0)
  (Actor|DestroyActor))

(event EventAttack
  (|CallParentFunction)
  (if (Variables|Default|GetCanAttack)
    (CallFunction|CorrecRotation)
    (Variables|Default|SetCanMove false)
    (Utilities|FlowControl|Delay (Math|Random|RandomFloatinRange (Variables|Default|Get最小攻击间隔) (Variables|Default|Get最大攻击间隔)))
    (if (not (Variables|Default|GetIsDeath))
      (Animation|Montage|PlayMontage (Variables|Character|GetMesh) (Variables|Default|GetAttackMontage)
        (:then
          (Variables|Default|SetCanAttack false))
        (:OnCompleted
          (Variables|Default|SetCanAttack true :!label _label)
          (Variables|Default|SetCanMove true))
        (:OnBlendOut
          (goto _label))
        (:OnInterrupted
          (goto _label))))))

(fn ConstructionScript)

(fn CalcLaunchVelocity
  (params (OtherActor :type Actor%20Object%20Reference))
  (Utilities|IsValid OtherActor
    (:Is%20Valid
      (if (>= (- (.y (Transformation|GetActorLocation OtherActor)) (.y (Transformation|GetActorLocation))) 0.0)
        (bind _output_get (LocalVariables|SetLaunch%20Velo "0.000000,-500.000000,0.000000"))
        (return _output_get)
        (else
          (bind _output_get_2 (LocalVariables|SetLaunch%20Velo "0.000000,500.000000,0.000000"))
          (return _output_get_2))))))

(fn CorrecRotation
  (bind _returnvalue (Transformation|GetActorRotation))
  (if (> (.y (Transformation|GetActorForwardVector)) 0.0)
    (Transformation|SetActorRotation (Math|Rotator|MakeRotator (.roll _returnvalue) (.pitch _returnvalue) 9e+01))
    (else
      (Transformation|SetActorRotation (Math|Rotator|MakeRotator (.roll _returnvalue) (.pitch _returnvalue) -9e+01)))))