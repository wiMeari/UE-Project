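; BP_RightMapBorder is a map-edge trigger that stops the player camera from following the character past the right border.
; Box overlap by BP_TPCharacter turns off CameraXYCanFollow on its BP_ProjPlayerController, and end overlap restores it.
; While the character is inside, Tick uses FInterpTo to ease the camera actor's Y toward the box's negative-Y edge, leaving X and Z unchanged.
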(event OnComponentEndOverlap(Box)
  (params (OverlappedComponent :type Primitive%20Component%20Object%20Reference) (OtherActor :type Actor%20Object%20Reference) (OtherComp :type Primitive%20Component%20Object%20Reference) (OtherBodyIndex :type Integer))
  (bind _asbp_tpcharacter (Utilities|Casting|CastToBP_TPCharacter OtherActor))
  (bind _asbp_proj_player_controller (Utilities|Casting|CastToBP_ProjPlayerController (Pawn|GetController _asbp_tpcharacter)))
  (Variables|/Script/TeamProject.ProjPlayerController|SetCameraXYCanFollow _asbp_proj_player_controller true)
  (Variables|Default|SetCharacterInBox false))

(event OnComponentBeginOverlap(Box)
  (params (OverlappedComponent :type Primitive%20Component%20Object%20Reference) (OtherActor :type Actor%20Object%20Reference) (OtherComp :type Primitive%20Component%20Object%20Reference) (OtherBodyIndex :type Integer) (bFromSweep :type Boolean) (SweepResult :type Hit%20Result%20Structure%20%28by%20ref%29))
  (bind _asbp_tpcharacter (Utilities|Casting|CastToBP_TPCharacter OtherActor))
  (bind _asbp_proj_player_controller (Utilities|Casting|CastToBP_ProjPlayerController (Pawn|GetController _asbp_tpcharacter)))
  (Variables|Default|SetAs%20BP%20Proj%20Player%20Controller _asbp_proj_player_controller)
  (Variables|/Script/TeamProject.ProjPlayerController|SetCameraXYCanFollow _asbp_proj_player_controller false)
  (Variables|Default|SetCharacterInBox true))

(event EventBeginPlay)

(event EventTick
  (params (DeltaSeconds :type Float%20%28single-precision%29))
  (Variables|Default|SetDelta%20Seconds DeltaSeconds)
  (if (Variables|Default|GetCharacterInBox)
    (bind _as_bp_proj_player_controller (Variables|Default|GetAs%20BP%20Proj%20Player%20Controller)
      (:then
        (Transformation|SetActorLocation (Variables|/Script/TeamProject.PlayerCameraController|GetPlayerCameraActor (Variables|/Game/T/Blueprint/Character/Controller/BP_ProjPlayerController.BP_ProjPlayerController_C|GetBP%20Camera%20Controller _as_bp_proj_player_controller)) (Math|Vector|MakeVector (.x (Transformation|GetActorLocation (Variables|/Script/TeamProject.PlayerCameraController|GetPlayerCameraActor (Variables|/Game/T/Blueprint/Character/Controller/BP_ProjPlayerController.BP_ProjPlayerController_C|GetBP%20Camera%20Controller _as_bp_proj_player_controller)))) (Math|Interpolation|FInterpTo (.y (Transformation|GetActorLocation (Variables|/Script/TeamProject.PlayerCameraController|GetPlayerCameraActor (Variables|/Game/T/Blueprint/Character/Controller/BP_ProjPlayerController.BP_ProjPlayerController_C|GetBP%20Camera%20Controller _as_bp_proj_player_controller)))) (- (.y (Transformation|GetActorLocation)) (.y (Components|Box|GetScaledBoxExtent (Variables|Default|GetBox)))) (Variables|Default|GetDelta%20Seconds) 4.0) (.z (Transformation|GetActorLocation (Variables|/Script/TeamProject.PlayerCameraController|GetPlayerCameraActor (Variables|/Game/T/Blueprint/Character/Controller/BP_ProjPlayerController.BP_ProjPlayerController_C|GetBP%20Camera%20Controller _as_bp_proj_player_controller))))) false false))
      (:else))))

(fn ConstructionScript)