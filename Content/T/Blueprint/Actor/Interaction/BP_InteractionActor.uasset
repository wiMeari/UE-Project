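; BP_InteractionActor is an interactable actor that shows a tip widget when a TPCharacter is nearby, with an empty Interact event.
; On BeginPlay it writes TipText into the WBP_TipOfInteractionActor hosted by its Widget component.
; Sphere begin and end overlaps with a TPCharacter play that widget's appear and disappear animations.
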(event OnComponentBeginOverlap(Sphere)
  (params (OverlappedComponent :type Primitive%20Component%20Object%20Reference) (OtherActor :type Actor%20Object%20Reference) (OtherComp :type Primitive%20Component%20Object%20Reference) (OtherBodyIndex :type Integer) (bFromSweep :type Boolean) (SweepResult :type Hit%20Result%20Structure%20%28by%20ref%29))
  (Utilities|Casting|CastToTPCharacter OtherActor)
  (bind _aswbp_tip_of_interaction_actor (Utilities|Casting|CastToWBP_TipOfInteractionActor (UserInterface|GetWidget (Variables|Default|GetWidget))))
  (Default|AnimAppear _aswbp_tip_of_interaction_actor))

(event OnComponentEndOverlap(Sphere)
  (params (OverlappedComponent :type Primitive%20Component%20Object%20Reference) (OtherActor :type Actor%20Object%20Reference) (OtherComp :type Primitive%20Component%20Object%20Reference) (OtherBodyIndex :type Integer))
  (Utilities|Casting|CastToTPCharacter OtherActor)
  (bind _aswbp_tip_of_interaction_actor (Utilities|Casting|CastToWBP_TipOfInteractionActor (UserInterface|GetWidget (Variables|Default|GetWidget))))
  (Default|AnimDisappear _aswbp_tip_of_interaction_actor))

(event EventBeginPlay
  (bind _aswbp_tip_of_interaction_actor (Utilities|Casting|CastToWBP_TipOfInteractionActor (UserInterface|GetWidget (Variables|Default|GetWidget))))
  (Variables|Default|SetAs%20WBP%20Tip%20Of%20Interaction%20Actor _aswbp_tip_of_interaction_actor)
  (Rendering|Components|TextRender|SetText (Variables|/Game/T/Blueprint/UI/WBP_TipOfInteractionActor.WBP_TipOfInteractionActor_C|GetText (Variables|Default|GetAs%20WBP%20Tip%20Of%20Interaction%20Actor)) (Variables|Default|GetTipText)))

(event Collision|EventActorBeginOverlap
  (params (OtherActor :type Actor%20Object%20Reference)))

(event EventTick
  (params (DeltaSeconds :type Float%20%28single-precision%29)))

(event EventInteract)

(fn ConstructionScript)