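; Player controller that implements a "switch sense" skill, moving the player between two vertically stacked versions of the scene.
; On BeginPlay it derives the height offset from two BP_CalcActors and passes it to BP_CameraController, which also receives UsingSkill every Tick.
; The skill input expands an MPC_Scene radius, then after a delay teleports the pawn by that offset and triggers the camera switch.
; The texture-restore sequence that clears UsingSkill is unconnected.
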(event Input|EnhancedActionEvents|EnhancedInputActionIA_SwitchSense
  (params (ActionValue :type Boolean) (ElapsedSeconds :type Float%20%28double-precision%29) (TriggeredSeconds :type Float%20%28double-precision%29) (InputAction :type Input%20Action%20Object%20Reference :default "/Game/T/Input/Actions/Skills/IA_SwitchSense.IA_SwitchSense"))
  (:Started
    (Variables|Default|SetUsingSkill true)
    (Rendering|Material|SetVectorParameterValue "/Game/T/Texture/Param/MPC_Scene.MPC_Scene" "Location" (Math|Conversions|ToLinearColor(Vector) (Variables|Default|GetPlayerLocation)) :!class /Script/Engine.KismetMaterialLibrary)
    (bind _新建轨道_2 (Timeline|时间轴 PlayFromStart)
      (:Update
        (Rendering|Material|SetScalarParameterValue "/Game/T/Texture/Param/MPC_Scene.MPC_Scene" "Radius" (Math|Float|Lerp 0.0 8e+03 _新建轨道_2) :!class /Script/Engine.KismetMaterialLibrary)
        (Rendering|Material|SetVectorParameterValue "/Game/T/Texture/Param/MPC_Scene.MPC_Scene" "Location" (Math|Conversions|ToLinearColor(Vector) (Variables|Default|GetPlayerLocation)) :!class /Script/Engine.KismetMaterialLibrary))
      (:Finished
        (Rendering|Material|SetScalarParameterValue "/Game/T/Texture/Param/MPC_Scene.MPC_Scene" "Radius" 0.0 :!class /Script/Engine.KismetMaterialLibrary)))))

(event Input|EnhancedActionEvents|EnhancedInputActionIA_SwitchSense
  (params (ActionValue :type Boolean) (ElapsedSeconds :type Float%20%28double-precision%29) (TriggeredSeconds :type Float%20%28double-precision%29) (InputAction :type Input%20Action%20Object%20Reference :default "/Game/T/Input/Actions/Skills/IA_SwitchSense.IA_SwitchSense"))
  (Utilities|FlowControl|Delay 0.5)
  (CallFunction|SwitchSenseSkill))

(event EventBeginPlay
  (CallFunction|UpdateSceneHeightDifference)
  (bind _playercameramanager (Variables|Default|GetPlayerCameraManager)
    (:then
      (bind _asbp_camera_controller (Utilities|Casting|CastToBP_CameraController _playercameramanager))
      (bind _output_get (Variables|Default|SetBP%20Camera%20Controller _asbp_camera_controller))
      (Variables|/Game/T/Character/Controller/BP_CameraController.BP_CameraController_C|SetCameraHeightDifference _output_get (Variables|地图参数|GetSceneHeightDifference)))
    (:else)))

(event EventTick
  (params (DeltaSeconds :type Float%20%28single-precision%29))
  (bind _bp_camera_controller (Variables|Default|GetBP%20Camera%20Controller)
    (:then
      (Variables|/Game/T/Character/Controller/BP_CameraController.BP_CameraController_C|SetUsingSkill _bp_camera_controller (Variables|Default|GetUsingSkill)))
    (:else)))

(fn ConstructionScript)

(fn UpdateSceneHeightDifference
  (bind _outactors (Actor|GetAllActorsOfClass "/Game/T/Actor/BP_CalcActor.BP_CalcActor_C"))
  (Utilities|IsValid (Utilities|Array|Get(acopy) _outactors 1)
    (:Is%20Valid
      (Utilities|IsValid (Utilities|Array|Get(acopy) _outactors)
        (:Is%20Valid
          (Variables|地图参数|SetSceneHeightDifference (Math|Float|Absolute(Float) (- (.z (Transformation|GetActorLocation (Utilities|Array|Get(acopy) _outactors 1))) (.z (Transformation|GetActorLocation (Utilities|Array|Get(acopy) _outactors)))))))))))

(fn SwitchSenseSkill
  (bind _returnvalue (Game|Player|GetPlayerPawn 0))
  (bind _playerlocation (Variables|Default|GetPlayerLocation))
  (bind _playerlocation_2 (Variables|Default|GetPlayerLocation))
  (bind _tpcharacter (Variables|Default|GetTPCharacter))
  (bind _returnvalue_2 (Transformation|GetActorTransform _tpcharacter))
  ;[0.15 0.15 0.15 0.5] 改变玩家位置
  (if (> (.z (Variables|Default|GetPlayerLocation)) (Variables|地图参数|GetSceneHeightDifference))
    (bind _output_get (Variables|Default|SetSwitchLocation (Math|Vector|MakeVector (.x _playerlocation_2) (.y _playerlocation_2) (- (.z _playerlocation_2) (Variables|地图参数|GetSceneHeightDifference)))))
    (Transformation|SetActorTransform _returnvalue (Math|Transform|MakeTransform _output_get (.rotation _returnvalue_2) (.scale _returnvalue_2)))
    (else
      (bind _output_get_2 (Variables|Default|SetSwitchLocation (Math|Vector|MakeVector (.x _playerlocation) (.y _playerlocation) (+ (.z _playerlocation) (Variables|地图参数|GetSceneHeightDifference)))))
      (Transformation|SetActorTransform _returnvalue (Math|Transform|MakeTransform _output_get_2 (.rotation _returnvalue_2) (.scale _returnvalue_2)))))
  (bind _playercameramanager (Variables|Default|GetPlayerCameraManager)
    (:then
      (bind _asbp_camera_controller (Utilities|Casting|CastToBP_CameraController _playercameramanager))
      (Default|EventCameraSwitch _asbp_camera_controller)
      (return))
    (:else)))