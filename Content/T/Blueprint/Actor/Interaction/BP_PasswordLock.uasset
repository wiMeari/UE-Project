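; An interactable password lock actor that opens a code-entry screen and triggers the next step once solved.
; On BeginPlay it creates a WBP_PasswordLock widget, adds it to the viewport and binds to its password-pass callback.
; Interact makes the widget visible, shows the mouse cursor and pauses the game.
; On a pass, it disables the Sphere's collision and calls CallNext.
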(event Custom|OnPasswordPass
  (Collision|SetCollisionEnabled (Variables|Default|GetSphere) "NoCollision")
  (Default|CallNext))

(event EventBeginPlay
  (|CallParentFunction)
  (bind _returnvalue (UserInterface|CreateWidget "/Game/T/Blueprint/UI/WBP_PasswordLock.WBP_PasswordLock_C" (Game|GetPlayerController 0)))
  (bind _output_get (Variables|Default|SetPassword _returnvalue))
  (UserInterface|Viewport|AddtoViewport _output_get 0)
  (EventDispatchers|AssignPasswordPass _returnvalue (EventDispatchers|CreateEvent :!event Custom|OnPasswordPass)))

(event Collision|EventActorBeginOverlap
  (params (OtherActor :type Actor%20Object%20Reference)))

(event EventTick
  (params (DeltaSeconds :type Float%20%28single-precision%29)))

(event EventInteract
  (Widget|SetVisibility (Variables|Default|GetPassword) "Visible")
  (Variables|/Script/Engine.PlayerController|SetbShowMouseCursor (Game|GetPlayerController 0) true)
  (Game|SetGamePaused true))

(fn ConstructionScript)