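; BP_Wall is an enemy wall that moves along world Y and deals effectively lethal damage to what it overlaps.
; After a BeginPlay delay it enables movement, then shortly afterwards plays a sound at its location.
; While enabled, Tick restarts a timeline every frame, whose update adds a lerped offset to the current Y position without sweeping.
; Box overlaps call GetHit on actors implementing CombatInterface, passing the wall's location as hit direction.
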(event OnComponentBeginOverlap(Box)
  (params (OverlappedComponent :type Primitive%20Component%20Object%20Reference) (OtherActor :type Actor%20Object%20Reference) (OtherComp :type Primitive%20Component%20Object%20Reference) (OtherBodyIndex :type Integer) (bFromSweep :type Boolean) (SweepResult :type Hit%20Result%20Structure%20%28by%20ref%29))
  (bind _ascombat_interface (Utilities|Casting|CastToCombatInterface OtherActor))
  (Class|CombatInterface|GetHit _ascombat_interface 9999999.0 (Transformation|GetActorLocation)))

(event EventBeginPlay
  (Utilities|FlowControl|Delay 1.0)
  (Variables|Default|SetCanMove true)
  (Utilities|FlowControl|Delay 0.7)
  (Audio|PlaySoundatLocation "/Game/D/Voice/MS_Level2Soun.MS_Level2Soun" (Transformation|GetActorLocation) "0, 0, 0" 1.0 1.0 0.0 0 0 0 0))

(event Collision|EventActorBeginOverlap
  (params (OtherActor :type Actor%20Object%20Reference)))

(event EventTick
  (params (DeltaSeconds :type Float%20%28single-precision%29))
  (bind _returnvalue (Transformation|GetActorLocation))
  (if (Variables|Default|GetCanMove)
    (bind _新建轨道_0 (Timeline|时间轴 PlayFromStart)
      (:Update
        (Transformation|SetActorLocation (Math|Vector|MakeVector (.x _returnvalue) (+ (Math|Float|Lerp 0.0 2.817e+04 _新建轨道_0) (.y _returnvalue)) (.z _returnvalue)) false false)))))

(fn ConstructionScript)