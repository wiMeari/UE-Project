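; BP_NextLevelDoor is a door actor that rises to open, apparently as the way to the next level.
; BeginPlay stores a target height 400 units above its start and binds to the Next dispatcher on a Lock reference.
; The Open event plays a timeline that lerps Z toward that target, blending from the current height each update rather than a fixed start.
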(event Custom|Open
  (bind _returnvalue (Transformation|GetActorLocation))
  (bind _新建轨道_0 (Timeline|时间轴 Play)
    (:Update
      (Transformation|SetActorLocation (Math|Vector|MakeVector (.x _returnvalue) (.y _returnvalue) (Math|Float|Lerp (.z (Transformation|GetActorLocation)) (Variables|Default|GetB) _新建轨道_0)) false false))))

(event EventBeginPlay
  (Variables|Default|SetB (+ (.z (Transformation|GetActorLocation)) 4e+02))
  (EventDispatchers|AssignNext (Variables|Default|GetLock) (EventDispatchers|CreateEvent :!event Custom|Open)))

(event Collision|EventActorBeginOverlap
  (params (OtherActor :type Actor%20Object%20Reference)))

(event EventTick
  (params (DeltaSeconds :type Float%20%28single-precision%29)))

(fn ConstructionScript)