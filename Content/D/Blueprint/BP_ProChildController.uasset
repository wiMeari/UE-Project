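; Child player controller that links the character to the HUD and handles pausing.
; On BeginPlay it runs parent logic, then passes a valid BPTPCharacter to the TPHUD.
; The P key toggles UI_Pause, cursor visibility and UI-only or game-only input, faking pause with heavy global time dilation rather than a true game pause.
; The IA_Pause input action event is empty.
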(event Input|EnhancedActionEvents|EnhancedInputActionIA_Pause
  (params (ActionValue :type Boolean) (ElapsedSeconds :type Float%20%28double-precision%29) (TriggeredSeconds :type Float%20%28double-precision%29) (InputAction :type Input%20Action%20Object%20Reference :default "/Game/T/Input/Actions/Base/IA_Pause.IA_Pause")))

(event EventBeginPlay
  (|CallParentFunction)
  (bind _bp_tpcharacter (Variables|Default|GetBP%20TPCharacter)
    (:then
      (bind _astphud (Utilities|Casting|CastToTPHUD (HUD|GetHUD)))
      (Variables|/Game/D/TPHUD.TPHUD_C|SetCharacter _astphud _bp_tpcharacter))
    (:else)))

(event EventTick
  (params (DeltaSeconds :type Float%20%28single-precision%29))
  (|CallParentFunction DeltaSeconds) ; 此节点被禁用，将不会被调用。\n从引脚连出引线来编译功能。
)

(event Input|KeyboardEvents|P
  (params (Key :type Key%20Structure :default "None"))
  (bind _returnvalue (Game|GetPlayerController 0))
  (:Pressed
    (if (Variables|Default|GetOn%20Paused)
      (Variables|Default|SetOn%20Paused false)
      (Widget|RemovefromParent (stale _returnvalue_2))
      (Variables|/Script/Engine.PlayerController|SetbShowMouseCursor _returnvalue false)
      (Input|SetInputModeGameOnly _returnvalue false)
      (Utilities|Time|SetGlobalTimeDilation 1.0)
      (else
        (Variables|Default|SetOn%20Paused true)
        (bind _returnvalue_2 (UserInterface|CreateWidget "/Game/D/UI/UI_Pause.UI_Pause_C" _returnvalue))
        (UserInterface|Viewport|AddtoViewport _returnvalue_2 0)
        (Variables|/Script/Engine.PlayerController|SetbShowMouseCursor _returnvalue true)
        (Input|SetInputModeUIOnly _returnvalue 0 "DoNotLock" false)
        (Utilities|Time|SetGlobalTimeDilation 0.05)))))

(fn ConstructionScript
  (|CallParentFunction))