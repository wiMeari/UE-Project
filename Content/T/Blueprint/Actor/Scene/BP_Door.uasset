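; BP_Door is a scene door actor that moves vertically along world Z when it receives an Interact event.
; Interact plays a timeline whose track drives a Lerp, feeding a Z offset into AddActorWorldOffset on each update.
; The offset accumulates per update, so total travel depends on update count as well as the curve.
; The graph has no closing or reverse logic.
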(event EventBeginPlay
  (|CallParentFunction) ; 此节点被禁用，将不会被调用。\n从引脚连出引线来编译功能。
)

(event Collision|EventActorBeginOverlap
  (params (OtherActor :type Actor%20Object%20Reference))
  (|CallParentFunction OtherActor) ; 此节点被禁用，将不会被调用。\n从引脚连出引线来编译功能。
)

(event EventTick
  (params (DeltaSeconds :type Float%20%28single-precision%29))
  (|CallParentFunction DeltaSeconds) ; 此节点被禁用，将不会被调用。\n从引脚连出引线来编译功能。
)

(event EventInteract
  (bind _新建轨道_0 (Timeline|时间轴 Play)
    (:Update
      (Transformation|AddActorWorldOffset (Math|Vector|MakeVector 0.0 0.0 (Math|Float|Lerp 0.0 1e+01 _新建轨道_0))))))

(fn ConstructionScript
  (|CallParentFunction))