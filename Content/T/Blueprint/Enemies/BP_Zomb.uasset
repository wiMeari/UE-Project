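; BP_Zomb is a zombie enemy Blueprint built on a parent class that supplies its death and hit handling.
; Each Tick, after calling the parent, it sets the movement component's max walk speed from IsChase, running fast while chasing and walking slowly otherwise.
; Death, GetHit and the construction script only forward to the parent, and the BeginPlay and overlap events are disabled stubs.
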(event EventBeginPlay
  (|CallParentFunction) ; 此节点被禁用，将不会被调用。\n从引脚连出引线来编译功能。
)

(event Collision|EventActorBeginOverlap
  (params (OtherActor :type Actor%20Object%20Reference))
  (|CallParentFunction OtherActor) ; 此节点被禁用，将不会被调用。\n从引脚连出引线来编译功能。
)

(event EventTick
  (params (DeltaSeconds :type Float%20%28single-precision%29))
  (bind _charactermovement (Variables|Character|GetCharacterMovement))
  (|CallParentFunction DeltaSeconds)
  (if (Variables|Default|GetIsChase)
    (Variables|/Script/Engine.CharacterMovementComponent|SetMaxWalkSpeed _charactermovement 5e+02)
    (else
      (Variables|/Script/Engine.CharacterMovementComponent|SetMaxWalkSpeed _charactermovement 125.0))))

(event EventDeath
  (|CallParentFunction))

(event EventGetHit
  (params (Damage :type Float%20%28single-precision%29) (HitDirection :type Vector%20%28by%20ref%29 :default "0, 0, 0") (Hitter :type Actor%20Object%20Reference))
  (|CallParentFunction Damage HitDirection Hitter))

(fn ConstructionScript
  (|CallParentFunction))