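; Third-person player character with melee combos, hit reaction, death notification and overlap-based interaction.
; Attack picks sprint, ground, air or plunge montages from movement state, stepping combos by AttackCount and randomly choosing the ground set at count zero.
; The plunge disables capsule collision and loops a timer into DownAttack until CanLaunchDownAttack triggers the landing section.
; A timeline dissolves the child-actor weapon between attacks, and Tick prints stamina for debugging.
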(event OnComponentBeginOverlap(InteractionBox)
  (params (OverlappedComponent :type Primitive%20Component%20Object%20Reference) (OtherActor :type Actor%20Object%20Reference) (OtherComp :type Primitive%20Component%20Object%20Reference) (OtherBodyIndex :type Integer) (bFromSweep :type Boolean) (SweepResult :type Hit%20Result%20Structure%20%28by%20ref%29))
  (bind _asinteraction (Utilities|Casting|CastToInteraction OtherActor))
  (Variables|交互|SetCanInteract true))

(event OnComponentEndOverlap(InteractionBox)
  (params (OverlappedComponent :type Primitive%20Component%20Object%20Reference) (OtherActor :type Actor%20Object%20Reference) (OtherComp :type Primitive%20Component%20Object%20Reference) (OtherBodyIndex :type Integer))
  (Utilities|Casting|CastToInteraction OtherActor)
  (Variables|交互|SetCanInteract false))

(event Custom|ComboReset
  (Variables|攻击数据|SetAttackCount 0))

(event Custom|BeginAttack
  (bind _新建轨道_0 (Timeline|时间轴 ReverseFromEnd)
    (:Update
      (Default|Dissolved (Variables|武器|GetWeapon%20Actor) _新建轨道_0))))

(event Custom|EndAttack
  (bind _新建轨道_0 (Timeline|时间轴 PlayFromStart)
    (:Update
      (Default|Dissolved (Variables|武器|GetWeapon%20Actor) _新建轨道_0))))

(event Custom|DownAttack
  (bind _charactermovement (Variables|Character|GetCharacterMovement))
  ;[0.15 0.15 0.15 0.5] 下批攻击动画
  (Variables|/Script/Engine.CharacterMovementComponent|SetGravityScale _charactermovement 3.0)
  (if (Variables|Default|GetCanLaunchDownAttack)
    (Utilities|Time|ClearTimerbyFunctionName 0 "DownAttack")
    (Variables|/Script/Engine.CharacterMovementComponent|SetGravityScale _charactermovement 1.0)
    (Collision|SetCollisionEnabled (Variables|Default|GetCapsuleComponent) "QueryAndPhysics")
    (Animation|Montage|PlayMontage (Variables|Character|GetMesh) (stale EventAttack _returnvalue) 1.0 0.0 "End"
      (:then
        (Variables|攻击数据|SetCanAttack false))
      (:OnCompleted
        (Variables|攻击数据|SetCanAttack true :!label _label))
      (:OnBlendOut
        (goto _label))
      (:OnInterrupted
        (goto _label)))))

(event Custom|InteractToActor
  (Class|Interaction|Interact (stale OnComponentBeginOverlap(InteractionBox) _asinteraction)))

(event EventBeginPlay
  (bind _asbp_base_weapon (Utilities|Casting|CastToBP_BaseWeapon (Variables|/Script/Engine.ChildActorComponent|GetChildActor (Variables|Default|GetWeaponComponent))))
  (bind _output_get (Variables|武器|SetWeapon%20Actor _asbp_base_weapon))
  (Variables|武器|SetWeapon%20Mesh (Variables|/Script/TeamProject.TPWeapon|GetWeaponMesh _output_get))
  (Default|Dissolved _output_get 1.0))

(event EventDeath
  (|CallParentFunction)
  (Default|CallPlayerDeath))

(event EventTick
  (params (DeltaSeconds :type Float%20%28single-precision%29))
  (CallFunction|SelectAttackArray)
  (Development|PrintString (Utilities|String|ToString(Float) (Class|TPAttributeComponent|GetStamina (Variables|Default|GetAttributeComponent)))))

(event EventGetHit
  (params (Damage :type Float%20%28single-precision%29) (HitDirection :type Vector%20%28by%20ref%29 :default "0, 0, 0") (Hitter :type Actor%20Object%20Reference))
  (|CallParentFunction Damage HitDirection Hitter)
  (Animation|Montage|PlayMontage (Variables|Character|GetMesh) "/Game/T/Blueprint/Anim/YLAnim/AM_YLGetHit.AM_YLGetHit"
    (:then
      (Variables|攻击数据|SetCanAttack false))
    (:OnCompleted
      (Variables|攻击数据|SetCanAttack true :!label _label))
    (:OnBlendOut
      (goto _label))))

(event EventAttack
  (bind _montage_array (Variables|攻击动画|GetMontage%20Array))
  (bind _sprint_attack_montage (Variables|攻击动画|GetSprint%20Attack%20Montage))
  (bind _air_attack_montage_array (Variables|攻击动画|GetAir%20Attack%20Montage%20Array))
  (|CallParentFunction)
  (if (or (Variables|攻击数据|GetCanAttack) (Variables|攻击数据|GetCanCancel))
    (if (AI|Components|NavMovement|IsFalling (Variables|Character|GetCharacterMovement))
      (if (Variables|Default|GetIsDown)
        (if (Variables|Default|GetCanDownAttack)
          ;[0.15 0.15 0.15 0.5] 下批攻击动画
          (bind (_isnotnull _returnvalue) (Class|TPFunctionLibrary|SelectMontagefromMontageArray (Variables|攻击动画|GetAirTo%20Floor%20Attack%20Montage%20Array)))
          (if _isnotnull
            (Animation|Montage|PlayMontage (Variables|Character|GetMesh) _returnvalue 1.0 0.0 "Start"
              (:then
                (Variables|攻击数据|SetCanAttack false :!label _label)
                (Collision|SetCollisionEnabled (Variables|Default|GetCapsuleComponent) "NoCollision")
                (Utilities|Time|SetTimerbyFunctionName 0 "DownAttack" (Utilities|Time|GetWorldDeltaSeconds) true))
              (:OnCompleted
                (goto _label))
              (:OnInterrupted
                (Variables|攻击数据|SetCanAttack true))))
          (else
            ;[0.15 0.15 0.15 0.5] 空中普通攻击动画
            (if (Utilities|Array|IsNotEmpty _air_attack_montage_array) :!label _label_2
              (bind _montage (CallFunction|PlayCombo _air_attack_montage_array))
              (Animation|Montage|PlayMontage (Variables|Character|GetMesh) _montage
                (:then
                  (Variables|攻击数据|SetCanAttack false))
                (:OnCompleted
                  (Variables|攻击数据|SetCanAttack true :!label _label_3))
                (:OnBlendOut
                  (goto _label_3))
                (:OnInterrupted
                  (goto _label_3))))))
        (else
          (goto _label_2)))
      (elif (Variables|Default|GetIsSprint)
        ;[0.15 0.15 0.15 0.5] 奔跑攻击动画
        (if (Utilities|Array|IsNotEmpty _sprint_attack_montage)
          (bind _montage_2 (CallFunction|PlayCombo _sprint_attack_montage))
          (Animation|Montage|PlayMontage (Variables|Character|GetMesh) _montage_2
            (:then
              (Variables|攻击数据|SetCanAttack false))
            (:OnCompleted
              (Variables|攻击数据|SetCanAttack true :!label _label_4))
            (:OnBlendOut
              (goto _label_4))
            (:OnInterrupted
              (goto _label_4))))
        (else
          ;[0.15 0.15 0.15 0.5] 地面攻击动画
          (if (Utilities|Array|IsNotEmpty _montage_array)
            (bind _montage_3 (CallFunction|PlayCombo _montage_array))
            (Animation|Montage|PlayMontage (Variables|Character|GetMesh) _montage_3
              (:then
                (Variables|攻击数据|SetCanAttack false))
              (:OnCompleted
                (Variables|攻击数据|SetCanAttack true :!label _label_5))
              (:OnBlendOut
                (goto _label_5))
              (:OnInterrupted
                (goto _label_5)))))))))

(fn ConstructionScript)

(fn RangeSelecAttackMontageArray
  (params (Select :type Map%20of%20Integers%20to%20Structs))
  (bind _returnvalue (Utilities|Map|Length Select))
  (bind _returnvalue_2 (Utilities|Map|Length Select))
  (bind _returnvalue_3 (Math|Random|RandomInteger _returnvalue))
  (bind (_value _returnvalue_4) (Utilities|Map|Find Select _returnvalue_2))
  (bind _returnvalue_5 (+ _returnvalue_3 1))
  (bind (_value_2 _returnvalue_6) (Utilities|Map|Find Select _returnvalue_5))
  (if (> _returnvalue 1)
    (if _returnvalue_6
      (return (Utilities|Struct|BreakUAttackMontage _value_2) true)
      (else
        (return 0 false)))
    (elif _returnvalue_4
      (return (Utilities|Struct|BreakUAttackMontage _value) true)
      (else
        (return 0 false)))))

(fn PlayCombo
  (params (MontageArray :type Array%20of%20Anim%20Montage%20Object%20References))
  (if (> (- (Utilities|Array|Length MontageArray) 1) 0)
    (LocalVariables|SetLocalAttackMontage (Utilities|Array|Get(acopy) MontageArray (Variables|攻击数据|GetAttackCount)))
    (bind _result (Math|Integer|IncrementInt (Variables|攻击数据|GetAttackCount))
      (:%20%20
        (Variables|攻击数据|SetAttackCount _result)
        (return (LocalVariables|GetLocalAttackMontage))))
    (else
      (return (Utilities|Array|Get(acopy) MontageArray)))))

(fn SelectAttackArray
  (if (== (Variables|攻击数据|GetAttackCount) 0)
    (bind (_montagearray _isnotnull) (CallFunction|RangeSelecAttackMontageArray (Variables|攻击动画|GetAttack%20Montage)))
    (if _isnotnull
      (Variables|攻击动画|SetMontage%20Array _montagearray)))
  (return))

(fn SelectAttack
  (params (AttackArray :type Array%20of%20Anim%20Montage%20Object%20References))
  (if (Utilities|Array|IsNotEmpty (Variables|攻击动画|GetAirTo%20Floor%20Attack%20Montage%20Array))
    _))