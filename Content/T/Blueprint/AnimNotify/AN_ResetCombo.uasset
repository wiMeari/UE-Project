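; Anim notify that resets the owning BP_TPCharacter's attack combo at a point in an animation.
; It calls ComboReset, then checks the player controller's PlayerNeedMove flag.
; When movement is needed, it blends out the current montage, ends the attack and allows the weapon to dissolve.
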(fn ReceivedNotify
  (params (MeshComp :type Skeletal%20Mesh%20Component%20Object%20Reference) (Animation :type Anim%20Sequence%20Base%20Object%20Reference) (EventReference :type Anim%20Notify%20Event%20Reference%20Structure%20%28by%20ref%29))
  (bind _asbp_tpcharacter (Utilities|Casting|CastToBP_TPCharacter (Components|GetOwner MeshComp)))
  (Default|ComboReset _asbp_tpcharacter)
  (bind _asbp_proj_player_controller (Utilities|Casting|CastToBP_ProjPlayerController (Pawn|GetController _asbp_tpcharacter)))
  (if (Variables|/Script/TeamProject.ProjPlayerController|GetPlayerNeedMove _asbp_proj_player_controller)
    (Animation|Montage|MontageStop (Components|SkeletalMesh|GetAnimInstance (Variables|/Script/Engine.Character|GetMesh _asbp_tpcharacter)) 0.5 0)
    (Default|EndAttack _asbp_tpcharacter)
    (Variables|/Game/T/Blueprint/Character/BP_TPCharacter.BP_TPCharacter_C|SetCanDissolvedWeapon _asbp_tpcharacter true)
    (return false)
    (else
      (return false))))